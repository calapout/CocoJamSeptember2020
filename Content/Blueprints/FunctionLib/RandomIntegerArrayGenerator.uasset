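; Blueprint function library with IntArrayGenerator, which builds a random integer array meant to represent numbers of likes.
; A while loop compares the array length to a random size between MinSize and MaxSize, drawn inside the loop condition.
; Its body adds a random value between MinValue and MaxValue, then returns the array from within the loop.
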(fn IntArrayGenerator
  (params (minSize :type Integer) (maxSize :type Integer))
  ;[1 1 1] Permits to randomize and array of ints that will represent the number of likes
  (while (< (Utilities|Array|Length (LocalVariables|GetintegerArray)) (Math|Random|RandomIntegerinRange minSize maxSize))
    (Utilities|Array|Add (LocalVariables|GetintegerArray) (Math|Random|RandomIntegerinRange (LocalVariables|GetminValue) (LocalVariables|GetmaxValue)))
    (return (LocalVariables|GetintegerArray))))