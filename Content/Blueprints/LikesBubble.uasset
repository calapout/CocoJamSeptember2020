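; LikesBubble is an actor that briefly shows a text popup with a random, fake "likes" count when play begins.
; ShowLikes makes the Nbre text visible and starts two timers.
; A looping timer rerolls the number every half second through ChangeValue, and a three-second one-shot hides the text and clears the looping timer.
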(event EventBeginPlay
  (Development|PrintString "Hello")
  (CallFunction|ShowLikes))

(event Collision|EventActorBeginOverlap
  (params (OtherActor :type Actor%20Object%20Reference)))

(event EventTick
  (params (DeltaSeconds :type Float%20%28single-precision%29)))

(fn ConstructionScript)

(fn ChangeValue
  (params (value :type Integer))
  (Rendering|Components|TextRender|SetText (Variables|Default|Getnbre) (Utilities|Text|ToText(String) (Utilities|String|Append "+ " (Utilities|String|ToString(Integer) value) " likes!"))))

(fn ShowLikes
  ;[1 1 1] object will appear
  (Rendering|SetVisibility (Variables|Default|Getnbre) true false)
  ;[1 1 1] object will disapear after 3 seconds
  (bind _returnvalue (Utilities|Time|SetTimerbyEvent (EventDispatchers|CreateEvent :!event LikesBubbleAutoGenFunc) 0.5 true))
  (Utilities|Time|SetTimerbyEvent (EventDispatchers|CreateEvent :!event LikesBubbleAutoGenFunc1) 3.0)
  (Variables|Default|SetfirstTimer _returnvalue))

(fn LikesBubbleAutoGenFunc
  ;[1 1 1] Randomize the number of likes
  (CallFunction|ChangeValue (Math|Random|RandomIntegerinRange 50 200000)))

(fn LikesBubbleAutoGenFunc1
  (Rendering|SetVisibility (Variables|Default|Getnbre) false false)
  (Utilities|Time|ClearandInvalidateTimerbyHandle (Variables|Default|GetfirstTimer)))